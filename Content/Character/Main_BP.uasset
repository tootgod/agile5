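; Main_BP is a character Blueprint that gives the player a timed shield ability on the right mouse button.
; When the game-time cooldown has expired, a press attaches the Shield_P emitter to the mesh, sets the Temp flag and starts a 20-second cooldown.
; A five-second timer calls SetNormalDamage to clear the flag, whose name suggests altered damage while shielded, though no damage logic appears here.
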(event `Key|RightMouseButton`
  (params (Key :type "Key Structure"))
  (bind _mesh (`self.Mesh`))
  (:`Pressed`
    (`/Engine/EditorBlueprintResources/StandardMacros.CompareFloat` (`self.Cooldown`) (`KismetSystemLibrary.GetGameTimeInSeconds`)
      (:`<`
        (`GameplayStatics.SpawnEmitterAttached` "/Game/Shield/Shield_P.Shield_P" _mesh "None" (`KismetMathLibrary.MakeVector` (.x (`SceneComponent.RelativeLocation` _mesh)) (.y (`SceneComponent.RelativeLocation` _mesh)) (+ (.z (`SceneComponent.RelativeLocation` _mesh)) 200.0)))
        (set `self.temp` true)
        (set `self.Cooldown` (+ (`KismetSystemLibrary.GetGameTimeInSeconds`) 20.0))
        (`KismetSystemLibrary.K2_SetTimer` null "SetNormalDamage" 5.0)))))

(fn `SetNormalDamage`
  (set `self.temp` false))

(fn `UserConstructionScript`)